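; BP_chocolate is a chocolate bar pickup that spins in the world until something overlaps it.
; Tick adds a fixed yaw step to the bar each frame, so spin speed depends on frame rate.
; The first overlap sets IsTriggered, which stops the spin, then hides the bar, disables its collision and plays a quiet 2D eating sound.
; The overlap does not filter the other actor, and the pickup actor is never destroyed.
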(event OnComponentBeginOverlap(chocolate_bar)
  (params (OverlappedComponent :type Primitive%20Component%20Object%20Reference) (OtherActor :type Actor%20Object%20Reference) (OtherComp :type Primitive%20Component%20Object%20Reference) (OtherBodyIndex :type Integer) (bFromSweep :type Boolean) (SweepResult :type Hit%20Result%20Structure%20%28by%20ref%29))
  (bind _chocolate_bar (Variables|Default|Getchocolate_bar))
  (if (not (Variables|Default|GetisTriggered))
    (Variables|Default|SetisTriggered true)
    (Rendering|SetVisibility _chocolate_bar false false)
    (Collision|SetCollisionEnabled _chocolate_bar "NoCollision")
    (Audio|PlaySound2D "/Game/eat.eat" 0.2 1.0 0.0 0 0)))

(event EventTick
  (params (DeltaSeconds :type Float%20%28single-precision%29))
  (bind _chocolate_bar (Variables|Default|Getchocolate_bar))
  (bind _returnvalue (Transformation|GetWorldRotation _chocolate_bar))
  (bind (_roll _pitch _yaw) (Math|Rotator|BreakRotator _returnvalue))
  (if (not (Variables|Default|GetisTriggered))
    (Transformation|SetWorldRotation (Variables|Default|Getchocolate_bar) (Math|Rotator|MakeRotator _roll _pitch (+ _yaw 1.0)) false false)))

(fn ConstructionScript)