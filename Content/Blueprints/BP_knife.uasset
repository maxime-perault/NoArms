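; BP_knife is a spinning knife pickup that turns up as part of a chocolate-door gag.
; Tick yaws the Knife component a fixed step per frame, independent of delta time.
; Any overlap, without checking the other actor, shows the player's knife, destroys Chocolate, changes and shifts the HolyChocolateDoor text to "No Arms, No Chocolate.", plays a pain sound and destroys the pickup.
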(event OnComponentBeginOverlap(knife)
  (params (OverlappedComponent :type Primitive%20Component%20Object%20Reference) (OtherActor :type Actor%20Object%20Reference) (OtherComp :type Primitive%20Component%20Object%20Reference) (OtherBodyIndex :type Integer) (bFromSweep :type Boolean) (SweepResult :type Hit%20Result%20Structure%20%28by%20ref%29))
  (bind _holychocolatedoor (Variables|Default|GetHolyChocolateDoor))
  (bind _textrender (Variables|/Script/Engine.TextRenderActor|GetTextRender _holychocolatedoor))
  (bind _returnvalue (Transformation|GetWorldLocation _textrender))
  (bind (_x _y _z) (Math|Vector|BreakVector _returnvalue))
  (bind _asfirst_person_character (Utilities|Casting|CastToFirstPersonCharacter (Game|Player|GetPlayerPawn 0)))
  (Default|SetKnifeVisibility _asfirst_person_character true)
  (Actor|DestroyActor (Variables|Default|GetChocolate))
  (Rendering|Components|TextRender|SetText _textrender (Utilities|Text|MakeLiteralText "No Arms, No Chocolate."))
  (Transformation|SetWorldLocation _textrender (Math|Vector|MakeVector (- _x 4e+01) _y _z) false false)
  (Audio|PlaySound2D "/Game/pain.pain" 0.2 1.0 0.0 0 0)
  (Actor|DestroyActor))

(event EventTick
  (params (DeltaSeconds :type Float%20%28single-precision%29))
  (bind _knife (Variables|Default|Getknife))
  (bind _returnvalue (Transformation|GetWorldRotation _knife))
  (bind (_roll _pitch _yaw) (Math|Rotator|BreakRotator _returnvalue))
  (Transformation|SetWorldRotation (Variables|Default|Getknife) (Math|Rotator|MakeRotator _roll _pitch (+ _yaw 1.0)) false false))

(fn ConstructionScript)