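; First_Enigma runs a puzzle step in which a one-time trigger rearranges the room and reveals a knife.
; On BeginPlay it hides the knife, disables its collision, and hides every wall except the first.
; Overlapping DoorTrigger disables it, removes the door and first two walls, and shows the remaining walls and a query-only knife.
; The same event rewrites two narrative texts and shifts the NarrativeWall text along Y.
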(event OnComponentBeginOverlap(DoorTrigger)
  (params (OverlappedComponent :type Primitive%20Component%20Object%20Reference) (OtherActor :type Actor%20Object%20Reference) (OtherComp :type Primitive%20Component%20Object%20Reference) (OtherBodyIndex :type Integer) (bFromSweep :type Boolean) (SweepResult :type Hit%20Result%20Structure%20%28by%20ref%29))
  (bind _narrative_wall (Variables|Default|GetNarrative%20wall))
  (bind _door (Variables|Default|GetDoor))
  (bind _knife (Variables|Default|Getknife))
  (bind _textrender (Variables|/Script/Engine.TextRenderActor|GetTextRender _narrative_wall))
  (bind _returnvalue (Transformation|GetWorldLocation _textrender))
  (bind (_x _y _z) (Math|Vector|BreakVector _returnvalue))
  (Collision|SetCollisionEnabled (Variables|Default|GetDoorTrigger) "NoCollision")
  (Rendering|Components|TextRender|SetText (Variables|/Script/Engine.TextRenderActor|GetTextRender (Variables|Default|GetWhy%20do%20you%20play%20blabla)) (Utilities|Text|MakeLiteralText "WHY do you play this game?"))
  (Rendering|Components|TextRender|SetText _textrender (Utilities|Text|MakeLiteralText "Still a narrative wall."))
  (Transformation|SetWorldLocation _textrender (Math|Vector|MakeVector _x (+ _y 1e+02) _z) false false)
  (Rendering|SetVisibility (Variables|/Script/Engine.StaticMeshActor|GetStaticMeshComponent _door) false false)
  (Collision|SetCollisionEnabled (Variables|/Script/Engine.StaticMeshActor|GetStaticMeshComponent _door) "NoCollision")
  (Collision|SetCollisionEnabled (Variables|/Game/Blueprints/BP_knife.BP_knife_C|Getknife _knife) "QueryOnly")
  (Rendering|SetVisibility (Variables|/Game/Blueprints/BP_knife.BP_knife_C|Getknife _knife) true false)
  (for (_array_element _array_index) (Variables|Default|GetWalls)
    (if (> _array_index 1)
      (Rendering|SetVisibility (Variables|/Script/Engine.StaticMeshActor|GetStaticMeshComponent _array_element) true false)
      (else
        (Rendering|SetVisibility (Variables|/Script/Engine.StaticMeshActor|GetStaticMeshComponent _array_element) false false)
        (Collision|SetCollisionEnabled (Variables|/Script/Engine.StaticMeshActor|GetStaticMeshComponent _array_element) "NoCollision")))))

(event EventBeginPlay
  (bind _knife (Variables|Default|Getknife))
  (Collision|SetCollisionEnabled (Variables|/Game/Blueprints/BP_knife.BP_knife_C|Getknife _knife) "NoCollision")
  (Rendering|SetVisibility (Variables|/Game/Blueprints/BP_knife.BP_knife_C|Getknife _knife) false false)
  (for (_array_element _array_index) (Variables|Default|GetWalls)
    (if (> _array_index 0)
      (Rendering|SetVisibility (Variables|/Script/Engine.StaticMeshActor|GetStaticMeshComponent _array_element) false false))))

(fn ConstructionScript)