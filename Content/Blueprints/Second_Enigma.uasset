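; Second enigma puzzle: four trigger volumes (south, north, west, east) shift a single opening around the walls as they are overlapped.
; CurrentOption enforces the cycle, with each valid overlap restoring one wall and removing the next's visibility and collision; the east wall is a separate DMWall.
; DrawCount stages joke texts over the first laps, then reveals an IdiotMove counter whose taunts escalate, eventually hinting at using the knife.
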(event OnComponentBeginOverlap(South)
  (params (OverlappedComponent :type Primitive%20Component%20Object%20Reference) (OtherActor :type Actor%20Object%20Reference) (OtherComp :type Primitive%20Component%20Object%20Reference) (OtherBodyIndex :type Integer) (bFromSweep :type Boolean) (SweepResult :type Hit%20Result%20Structure%20%28by%20ref%29))
  (bind _walls (Variables|Default|GetWalls))
  (bind _walls_2 (Variables|Default|GetWalls))
  (bind _output (Utilities|Array|Get(acopy) _walls))
  (bind _output_2 (Utilities|Array|Get(acopy) _walls_2 1))
  (bind _staticmeshcomponent (Variables|/Script/Engine.StaticMeshActor|GetStaticMeshComponent _output))
  (bind _staticmeshcomponent_2 (Variables|/Script/Engine.StaticMeshActor|GetStaticMeshComponent _output_2))
  (if (== (Variables|Default|Getcurrent_option) 0)
    (Rendering|SetVisibility _staticmeshcomponent true false)
    (Collision|SetCollisionEnabled _staticmeshcomponent "QueryAndPhysics")
    (Rendering|SetVisibility _staticmeshcomponent_2 false false)
    (Collision|SetCollisionEnabled _staticmeshcomponent_2 "NoCollision")
    (Variables|Default|Setcurrent_option 1)
    (Math|Integer|IncrementInt (Variables|Default|Getnb_walls_spawn)
      (:%20%20
        (if (== (Variables|Default|GetDrawCount) 2)
          (Rendering|SetVisibility (Variables|/Script/Engine.TextRenderActor|GetTextRender (Variables|Default|GetCounter)) true false)
          (Math|Integer|IncrementInt (Variables|Default|GetDrawCount)
            (:%20%20
              _)))
        (Math|Integer|IncrementInt (Variables|Default|GetidiotMove)
          (:%20%20
            (if (>= (Variables|Default|GetidiotMove) 10)
              (if (>= (Variables|Default|GetidiotMove) 20)
                (Rendering|Components|TextRender|SetText (Variables|/Script/Engine.TextRenderActor|GetTextRender (Variables|Default|GetCounter)) (Utilities|Text|ToText(String) (Utilities|String|Append (Utilities|String|MakeLiteralString "Ok, I lied, I'm a busy wall... 
You have to use your knife somewhere. 
All the walls can't waste their time like you do... 
 
Counter of stupid moves: ") (Utilities|String|ToString(Integer) (Variables|Default|GetidiotMove)))))
                (else
                  (Rendering|Components|TextRender|SetText (Variables|/Script/Engine.TextRenderActor|GetTextRender (Variables|Default|GetCounter)) (Utilities|Text|ToText(String) (Utilities|String|Append (Utilities|String|MakeLiteralString "You know, I'm a wall, 
I can stay here for years...  
 
 
Counter of stupid moves: ") (Utilities|String|ToString(Integer) (Variables|Default|GetidiotMove)))))))
              (else
                (Rendering|Components|TextRender|SetText (Variables|/Script/Engine.TextRenderActor|GetTextRender (Variables|Default|GetCounter)) (Utilities|Text|ToText(String) (Utilities|String|Append (Utilities|String|MakeLiteralString "For some people, wasting time  
to find some optional ways is  
an achievement by itself. 
 
Counter of stupid moves: ") (Utilities|String|ToString(Integer) (Variables|Default|GetidiotMove)))))))))))))

(event OnComponentBeginOverlap(North)
  (params (OverlappedComponent :type Primitive%20Component%20Object%20Reference) (OtherActor :type Actor%20Object%20Reference) (OtherComp :type Primitive%20Component%20Object%20Reference) (OtherBodyIndex :type Integer) (bFromSweep :type Boolean) (SweepResult :type Hit%20Result%20Structure%20%28by%20ref%29))
  (bind _walls (Variables|Default|GetWalls))
  (bind _walls_2 (Variables|Default|GetWalls))
  (bind _output (Utilities|Array|Get(acopy) _walls 1))
  (bind _output_2 (Utilities|Array|Get(acopy) _walls_2 2))
  (bind _staticmeshcomponent (Variables|/Script/Engine.StaticMeshActor|GetStaticMeshComponent _output))
  (bind _staticmeshcomponent_2 (Variables|/Script/Engine.StaticMeshActor|GetStaticMeshComponent _output_2))
  (if (== (Variables|Default|Getcurrent_option) 1)
    (Rendering|SetVisibility _staticmeshcomponent true false)
    (Collision|SetCollisionEnabled _staticmeshcomponent "QueryAndPhysics")
    (Rendering|SetVisibility _staticmeshcomponent_2 false false)
    (Collision|SetCollisionEnabled _staticmeshcomponent_2 "NoCollision")
    (Variables|Default|Setcurrent_option 2)
    (Math|Integer|IncrementInt (Variables|Default|Getnb_walls_spawn)
      (:%20%20
        (Math|Integer|IncrementInt (Variables|Default|GetidiotMove)
          (:%20%20
            (if (>= (Variables|Default|GetidiotMove) 10)
              (if (>= (Variables|Default|GetidiotMove) 20)
                (Rendering|Components|TextRender|SetText (Variables|/Script/Engine.TextRenderActor|GetTextRender (Variables|Default|GetCounter)) (Utilities|Text|ToText(String) (Utilities|String|Append (Utilities|String|MakeLiteralString "Ok, I lied, I'm a busy wall... 
You have to use your knife somewhere. 
All the walls can't waste their time like you do... 
 
Counter of stupid moves: ") (Utilities|String|ToString(Integer) (Variables|Default|GetidiotMove)))))
                (else
                  (Rendering|Components|TextRender|SetText (Variables|/Script/Engine.TextRenderActor|GetTextRender (Variables|Default|GetCounter)) (Utilities|Text|ToText(String) (Utilities|String|Append (Utilities|String|MakeLiteralString "You know, I'm a wall, 
I can stay here for years...  
 
 
Counter of stupid moves: ") (Utilities|String|ToString(Integer) (Variables|Default|GetidiotMove)))))))
              (else
                (Rendering|Components|TextRender|SetText (Variables|/Script/Engine.TextRenderActor|GetTextRender (Variables|Default|GetCounter)) (Utilities|Text|ToText(String) (Utilities|String|Append (Utilities|String|MakeLiteralString "For some people, wasting time  
to find some optional ways is  
an achievement by itself. 
 
Counter of stupid moves: ") (Utilities|String|ToString(Integer) (Variables|Default|GetidiotMove)))))))))))))

(event OnComponentBeginOverlap(West)
  (params (OverlappedComponent :type Primitive%20Component%20Object%20Reference) (OtherActor :type Actor%20Object%20Reference) (OtherComp :type Primitive%20Component%20Object%20Reference) (OtherBodyIndex :type Integer) (bFromSweep :type Boolean) (SweepResult :type Hit%20Result%20Structure%20%28by%20ref%29))
  (bind _walls (Variables|Default|GetWalls))
  (bind _dm_wall (Variables|Default|GetDM_Wall))
  (bind _output (Utilities|Array|Get(acopy) _walls 2))
  (bind _cube_dm (Variables|/Game/Blueprints/BP_DestructibleMesh.BP_DestructibleMesh_C|GetCube_DM _dm_wall))
  (bind _staticmeshcomponent (Variables|/Script/Engine.StaticMeshActor|GetStaticMeshComponent _output))
  (if (== (Variables|Default|Getcurrent_option) 2)
    (Rendering|SetVisibility _staticmeshcomponent true false)
    (Collision|SetCollisionEnabled _staticmeshcomponent "QueryAndPhysics")
    (Rendering|SetVisibility _cube_dm false false)
    (Collision|SetCollisionEnabled _cube_dm "NoCollision")
    (Variables|Default|Setcurrent_option 3)
    (Math|Integer|IncrementInt (Variables|Default|Getnb_walls_spawn)
      (:%20%20
        (if (== (Variables|Default|GetDrawCount) 0)
          (Rendering|SetVisibility (Variables|/Script/Engine.TextRenderActor|GetTextRender (Variables|Default|GetNot%20funny)) true false)
          (Math|Integer|IncrementInt (Variables|Default|GetDrawCount)
            (:%20%20
              _)))
        (Math|Integer|IncrementInt (Variables|Default|GetidiotMove)
          (:%20%20
            (if (>= (Variables|Default|GetidiotMove) 10)
              (if (>= (Variables|Default|GetidiotMove) 20)
                (Rendering|Components|TextRender|SetText (Variables|/Script/Engine.TextRenderActor|GetTextRender (Variables|Default|GetCounter)) (Utilities|Text|ToText(String) (Utilities|String|Append (Utilities|String|MakeLiteralString "Ok, I lied, I'm a busy wall... 
You have to use your knife somewhere. 
All the walls can't waste their time like you do... 
 
Counter of stupid moves: ") (Utilities|String|ToString(Integer) (Variables|Default|GetidiotMove)))))
                (else
                  (Rendering|Components|TextRender|SetText (Variables|/Script/Engine.TextRenderActor|GetTextRender (Variables|Default|GetCounter)) (Utilities|Text|ToText(String) (Utilities|String|Append (Utilities|String|MakeLiteralString "You know, I'm a wall, 
I can stay here for years...  
 
 
Counter of stupid moves: ") (Utilities|String|ToString(Integer) (Variables|Default|GetidiotMove)))))))
              (else
                (Rendering|Components|TextRender|SetText (Variables|/Script/Engine.TextRenderActor|GetTextRender (Variables|Default|GetCounter)) (Utilities|Text|ToText(String) (Utilities|String|Append (Utilities|String|MakeLiteralString "For some people, wasting time  
to find some optional ways is  
an achievement by itself. 
 
Counter of stupid moves: ") (Utilities|String|ToString(Integer) (Variables|Default|GetidiotMove)))))))))))))

(event OnComponentBeginOverlap(East)
  (params (OverlappedComponent :type Primitive%20Component%20Object%20Reference) (OtherActor :type Actor%20Object%20Reference) (OtherComp :type Primitive%20Component%20Object%20Reference) (OtherBodyIndex :type Integer) (bFromSweep :type Boolean) (SweepResult :type Hit%20Result%20Structure%20%28by%20ref%29))
  (bind _dm_wall (Variables|Default|GetDM_Wall))
  (bind _walls (Variables|Default|GetWalls))
  (bind _output (Utilities|Array|Get(acopy) _walls))
  (bind _cube_dm (Variables|/Game/Blueprints/BP_DestructibleMesh.BP_DestructibleMesh_C|GetCube_DM _dm_wall))
  (bind _staticmeshcomponent (Variables|/Script/Engine.StaticMeshActor|GetStaticMeshComponent _output))
  (if (== (Variables|Default|Getcurrent_option) 3)
    (Rendering|SetVisibility _cube_dm true false)
    (Collision|SetCollisionEnabled _cube_dm "QueryAndPhysics")
    (Rendering|SetVisibility _staticmeshcomponent false false)
    (Collision|SetCollisionEnabled _staticmeshcomponent "NoCollision")
    (Variables|Default|Setcurrent_option 0)
    (Math|Integer|IncrementInt (Variables|Default|Getnb_walls_spawn)
      (:%20%20
        (if (== (Variables|Default|GetDrawCount) 1)
          (Rendering|SetVisibility (Variables|/Script/Engine.TextRenderActor|GetTextRender (Variables|Default|GetJokes)) false false)
          (Rendering|SetVisibility (Variables|/Script/Engine.TextRenderActor|GetTextRender (Variables|Default|GetNot%20funny)) false false)
          (Variables|Default|SetidiotMove (- (Variables|Default|GetidiotMove) 4))
          (Math|Integer|IncrementInt (Variables|Default|GetDrawCount)
            (:%20%20
              _)))
        (Math|Integer|IncrementInt (Variables|Default|GetidiotMove)
          (:%20%20
            (if (>= (Variables|Default|GetidiotMove) 10)
              (if (>= (Variables|Default|GetidiotMove) 20)
                (Rendering|Components|TextRender|SetText (Variables|/Script/Engine.TextRenderActor|GetTextRender (Variables|Default|GetCounter)) (Utilities|Text|ToText(String) (Utilities|String|Append (Utilities|String|MakeLiteralString "Ok, I lied, I'm a busy wall... 
You have to use your knife somewhere. 
All the walls can't waste their time like you do... 
 
Counter of stupid moves: ") (Utilities|String|ToString(Integer) (Variables|Default|GetidiotMove)))))
                (else
                  (Rendering|Components|TextRender|SetText (Variables|/Script/Engine.TextRenderActor|GetTextRender (Variables|Default|GetCounter)) (Utilities|Text|ToText(String) (Utilities|String|Append (Utilities|String|MakeLiteralString "You know, I'm a wall, 
I can stay here for years...  
 
 
Counter of stupid moves: ") (Utilities|String|ToString(Integer) (Variables|Default|GetidiotMove)))))))
              (else
                (Rendering|Components|TextRender|SetText (Variables|/Script/Engine.TextRenderActor|GetTextRender (Variables|Default|GetCounter)) (Utilities|Text|ToText(String) (Utilities|String|Append (Utilities|String|MakeLiteralString "For some people, wasting time  
to find some optional ways is  
an achievement by itself. 
 
Counter of stupid moves: ") (Utilities|String|ToString(Integer) (Variables|Default|GetidiotMove)))))))))))))

(event EventBeginPlay
  (bind _walls (Variables|Default|GetWalls))
  (bind _output (Utilities|Array|Get(acopy) _walls))
  (bind _staticmeshcomponent (Variables|/Script/Engine.StaticMeshActor|GetStaticMeshComponent _output))
  ;[1 1 1] Array order: south, north, west, east
  (Rendering|SetVisibility _staticmeshcomponent false false)
  (Collision|SetCollisionEnabled _staticmeshcomponent "NoCollision")
  (Rendering|SetVisibility (Variables|/Script/Engine.TextRenderActor|GetTextRender (Variables|Default|GetNot%20funny)) false false)
  (Rendering|SetVisibility (Variables|/Script/Engine.TextRenderActor|GetTextRender (Variables|Default|GetCounter)) false false))

(fn ConstructionScript)