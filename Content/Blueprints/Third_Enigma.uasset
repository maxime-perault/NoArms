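; Third puzzle trigger that makes a hidden door and a text message appear when something enters its DoorTrigger volume.
; On BeginPlay it hides the referenced Door and Text and turns off the door's collision.
; The first overlap shows both and restores the door's query and physics collision, with an IsTriggered flag making the reveal one-shot.
; The overlap does not filter which actor enters.
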(event OnComponentBeginOverlap(DoorTrigger)
  (params (OverlappedComponent :type Primitive%20Component%20Object%20Reference) (OtherActor :type Actor%20Object%20Reference) (OtherComp :type Primitive%20Component%20Object%20Reference) (OtherBodyIndex :type Integer) (bFromSweep :type Boolean) (SweepResult :type Hit%20Result%20Structure%20%28by%20ref%29))
  (bind _door (Variables|Default|GetDoor))
  (bind _staticmeshcomponent (Variables|/Script/Engine.StaticMeshActor|GetStaticMeshComponent _door))
  (if (not (Variables|Default|GetisTriggered))
    (Variables|Default|SetisTriggered true)
    (Rendering|SetVisibility _staticmeshcomponent true false)
    (Collision|SetCollisionEnabled _staticmeshcomponent "QueryAndPhysics")
    (Rendering|SetVisibility (Variables|/Script/Engine.TextRenderActor|GetTextRender (Variables|Default|GetText)) true false)))

(event EventBeginPlay
  (bind _door (Variables|Default|GetDoor))
  (bind _staticmeshcomponent (Variables|/Script/Engine.StaticMeshActor|GetStaticMeshComponent _door))
  (Rendering|SetVisibility _staticmeshcomponent false false)
  (Collision|SetCollisionEnabled _staticmeshcomponent "NoCollision")
  (Rendering|SetVisibility (Variables|/Script/Engine.TextRenderActor|GetTextRender (Variables|Default|GetText)) false false))

(fn ConstructionScript)