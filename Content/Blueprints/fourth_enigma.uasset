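; Blueprint actor for the fourth enigma that reveals a wall and a text when its Box trigger is overlapped.
; On BeginPlay it hides the referenced Wall mesh and Text render and disables the wall's collision.
; The first overlap disables the Box's collision so it fires once, then shows both and makes the wall solid with query and physics collision.
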(event OnComponentBeginOverlap(Box)
  (params (OverlappedComponent :type Primitive%20Component%20Object%20Reference) (OtherActor :type Actor%20Object%20Reference) (OtherComp :type Primitive%20Component%20Object%20Reference) (OtherBodyIndex :type Integer) (bFromSweep :type Boolean) (SweepResult :type Hit%20Result%20Structure%20%28by%20ref%29))
  (bind _wall (Variables|Default|Getwall))
  (bind _staticmeshcomponent (Variables|/Script/Engine.StaticMeshActor|GetStaticMeshComponent _wall))
  (Collision|SetCollisionEnabled (Variables|Default|GetBox) "NoCollision")
  (Rendering|SetVisibility _staticmeshcomponent true false)
  (Collision|SetCollisionEnabled _staticmeshcomponent "QueryAndPhysics")
  (Rendering|SetVisibility (Variables|/Script/Engine.TextRenderActor|GetTextRender (Variables|Default|Gettext)) true false))

(event EventBeginPlay
  (bind _wall (Variables|Default|Getwall))
  (bind _staticmeshcomponent (Variables|/Script/Engine.StaticMeshActor|GetStaticMeshComponent _wall))
  (Rendering|SetVisibility _staticmeshcomponent false false)
  (Collision|SetCollisionEnabled _staticmeshcomponent "NoCollision")
  (Rendering|SetVisibility (Variables|/Script/Engine.TextRenderActor|GetTextRender (Variables|Default|Gettext)) false false))

(fn ConstructionScript)